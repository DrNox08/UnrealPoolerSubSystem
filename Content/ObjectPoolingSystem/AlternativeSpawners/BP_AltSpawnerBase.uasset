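; Alternative spawner base for the object pooling system, which prepares a pool of projectile actors at BeginPlay.
; It takes the spawner mesh and projectile class from SpawnerData, applies the mesh to its StaticMesh and creates the pool from that class.
; It then caches the projectile struct from a data table by RowName, printing a warning when the row is missing.
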(event EventBeginPlay
  (bind _spawner_data (Variables|Default|GetSpawner%20Data))
  ;[0.15 0.15 0.15 0.5] Set Spawner Mesh && Create Pool
  (Components|StaticMesh|SetStaticMesh (Variables|Default|GetStaticMesh) (Utilities|ResolveSoftReference (Class|ProjectileDataAsset|GetSpawnerMesh _spawner_data)))
  (bind _output_get (Variables|Default|SetActorToSpawn (Class|ProjectileDataAsset|GetProjectileBaseClass _spawner_data)))
  (CallFunction|CreateObjectPool _output_get)
  ;[0.15 0.15 0.15 0.5] Get Projectile data and save the requested struct from table
  (bind _returnvalue (Utilities|GetDataTableRow (Variables|Default|GetProjectile%20DataTable) (Variables|Default|GetRow%20Name))
    (:then
      (Variables|Default|SetProjectile%20Data _returnvalue))
    (:RowNotFound
      (Development|PrintString (Utilities|String|Append (Utilities|GetDisplayName self) "NOT FOUND IN DATA TABLE")))))

(fn ConstructionScript)