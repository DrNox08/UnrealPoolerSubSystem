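; Pooled projectile actor that starts hidden and flies straight forward once activated from the object pool.
; Activation data sets its damage, sphere material and transform, then reveals it and starts a five-second lifetime timer.
; While active, Tick moves it by speed along its forward vector without sweeping.
; Deactivation returns it to the pool and hides it, and a helper can move it to a visible deactivation pool.
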(event Custom|Set%20Projectile
  (params (Damage :type Float%20%28double-precision%29) (Material :type Material%20Instance%20Object%20Reference))
  ;[0.15 0.15 0.15 0.5] Set Damage and Material
  (Variables|Default|SetDamage Damage)
  (Variables|Default|SetMaterial Material))

(event EventActivate
  (params (ObjectPoolActivationData :type Objec%20Pool%20Activation%20Data%20Structure))
  ;[0.15 0.15 0.15 0.5] Activation Event
  (Variables|Default|SetDamage (.damage ObjectPoolActivationData))
  (Variables|Default|SetMaterial (.materialinstance ObjectPoolActivationData))
  (CallFunction|SetGraphics)
  (Transformation|SetActorTransform (.objectpooltransform ObjectPoolActivationData))
  (bind _returnvalue (Utilities|Time|SetTimerbyEvent (EventDispatchers|CreateEvent :!event Deactivate) 5.0))
  (Variables|Default|SetDeactivateLifeTimerHandle _returnvalue)
  (Variables|Default|SetIs%20Active%20Projectile true)
  (Rendering|SetActorHiddenInGame false))

(event EventDeactivate
  (params (ObjectPoolDeactivationData :type Object%20Pool%20Deactivation%20Data%20Structure))
  (bind _self self)
  ;[0.15 0.15 0.15 0.5] Deactivation Event
  (CallFunction|ReturnProjectiletoPool (Utilities|GetClass _self) _self)
  (Rendering|SetActorHiddenInGame true))

(event EventTick
  (params (DeltaSeconds :type Float%20%28single-precision%29))
  ;[0.15 0.15 0.15 0.5] Move the object forward
  (if (Variables|Default|GetIs%20Active%20Projectile)
    (CallFunction|IncreaseXValue DeltaSeconds)))

(event EventBeginPlay
  (Rendering|SetActorHiddenInGame true))

(fn ConstructionScript)

(fn SetGraphics
  (bind _returnvalue (Rendering|Material|CreateDynamicMaterialInstance (Variables|Default|GetSphere) 0 (Variables|Default|GetMaterial) "None" :!class /Script/Engine.PrimitiveComponent))
  (Rendering|Material|SetMaterial (Variables|Default|GetSphere) 0 _returnvalue))

(fn IncreaseXValue
  (params (Delta%20Time :type Float%20%28single-precision%29))
  (Transformation|SetActorLocation (+ (* (* (Variables|Default|GetSpeed) (Transformation|GetActorForwardVector)) Delta%20Time) (Transformation|GetActorLocation)) false false))

(fn Deactivate
  (Class|Poolable|Deactivate))

(fn MoveActortoVisiblePool
  (Transformation|SetActorLocation (Transformation|GetActorLocation (Variables|Default|GetVisible%20Deactivation%20Pool)) false false)
  (CallFunction|SetGraphics))