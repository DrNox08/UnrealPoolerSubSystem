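; Base poolable projectile that flies forward while active and returns to the object pool on deactivation.
; Activation places it at the supplied transform, switches its dynamic material to the active color and starts a lifetime timer; Tick moves it without sweeping.
; Instead of being hidden, inactive projectiles move to the visible pool actor found at BeginPlay and switch to the deactivation color, keeping pooling visible in game.
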(event EventDeactivate
  (params (ObjectPoolDeactivationData :type Object%20Pool%20Deactivation%20Data%20Structure))
  (bind _self self)
  (CallFunction|ReturnProjectiletoPool (Utilities|GetClass _self) _self)
  ;[0.15 0.15 0.15 0.5 17] Keep the actor active in game changing it's color
  (CallFunction|MoveActortoVisiblePool)
  (Variables|Default|SetIs%20Active%20Projectile false))

(event EventActivate
  (params (ObjectPoolActivationData :type Objec%20Pool%20Activation%20Data%20Structure))
  (CallFunction|SetGraphics true)
  (Transformation|SetActorTransform (Math|Transform|MakeTransform (.location (.objectpooltransform ObjectPoolActivationData)) (.rotation (.objectpooltransform ObjectPoolActivationData)) "1.000000,1.000000,1.000000"))
  (bind _returnvalue (Utilities|Time|SetTimerbyEvent (EventDispatchers|CreateEvent :!event Deactivate) 5.0))
  (Variables|Default|SetDeactivateLifeTimerHandle _returnvalue)
  (Variables|Default|SetIs%20Active%20Projectile true))

(event EventTick
  (params (DeltaSeconds :type Float%20%28single-precision%29))
  (if (Variables|Default|GetIs%20Active%20Projectile)
    (CallFunction|IncreaseXValue DeltaSeconds)))

(event EventBeginPlay
  (bind _returnvalue (Actor|GetActorOfClass "/Game/ObjectPoolingSystem/Projectiles/Bp_ProjectilesVisiblePool.Bp_ProjectilesVisiblePool_C"))
  (Variables|Default|SetVisible%20Deactivation%20Pool _returnvalue)
  (CallFunction|MoveActortoVisiblePool))

(fn ConstructionScript)

(fn SetGraphics
  (params (Is%20Active :type Boolean))
  (Utilities|IsValid (Variables|Default|GetMaterial)
    (:Is%20Valid
      _)
    (:Is%20Not%20Valid
      (bind _returnvalue (Rendering|Material|CreateDynamicMaterialInstance (Variables|Default|GetSphere) 0 (Rendering|Material|GetMaterial (Variables|Default|GetSphere) 0) "None" :!class /Script/Engine.PrimitiveComponent))
      (Variables|Default|SetMaterial _returnvalue)))
  (if Is%20Active
    (Rendering|Material|SetVectorParameterValue (Variables|Default|GetMaterial) "Color" (Variables|Default|GetActivation%20Color) :!class /Script/Engine.MaterialInstanceDynamic)
    (else
      (Rendering|Material|SetVectorParameterValue (Variables|Default|GetMaterial) "Color" (Variables|Default|GetDeactivation%20Color) :!class /Script/Engine.MaterialInstanceDynamic))))

(fn IncreaseXValue
  (params (Delta%20Time :type Float%20%28single-precision%29))
  (Transformation|SetActorLocation (+ (* (* (Variables|Default|GetSpeed) (Transformation|GetActorForwardVector)) Delta%20Time) (Transformation|GetActorLocation)) false false))

(fn Deactivate
  (Class|Poolable|Deactivate))

(fn MoveActortoVisiblePool
  (Transformation|SetActorLocation (Transformation|GetActorLocation (Variables|Default|GetVisible%20Deactivation%20Pool)) false false)
  (CallFunction|SetGraphics false))