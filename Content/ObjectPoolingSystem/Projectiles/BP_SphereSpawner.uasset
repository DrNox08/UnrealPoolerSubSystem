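; BP_SphereSpawner is a timed spawner that emits BP_SpawnableSphere2 instances from an object pool.
; It creates the pool on BeginPlay, then accumulates delta time on Tick until the spawn interval is reached.
; At each interval it resets the timer, takes a pooled sphere, activates it at the spawner's location and prints a debug message.
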(event EventBeginPlay
  (CallFunction|CreateObjectPool "/Game/ObjectPoolingSystem/Projectiles/BP_SpawnableSphere2.BP_SpawnableSphere2_C"))

(event EventTick
  (params (DeltaSeconds :type Float%20%28single-precision%29))
  ;[0.15 0.15 0.15 0.5] Controlla se é trascorso lo Spawn Interval
  (Variables|Default|SetElapsedTime (+ DeltaSeconds (Variables|Default|GetElapsedTime)))
  (if (>= (Variables|Default|GetElapsedTime) (Variables|Default|GetSpawnInterval))
    (Variables|Default|SetElapsedTime 0.0)
    (bind _poolable_actor (CallFunction|GetProjectilefromPool "/Game/ObjectPoolingSystem/Projectiles/BP_SpawnableSphere2.BP_SpawnableSphere2_C"))
    (Class|Poolable|Activate _poolable_actor (Utilities|Struct|MakeObjecPoolActivationData (Math|Transform|MakeTransform (Transformation|GetActorLocation) "0, 0, 0" "1.000000,1.000000,1.000000") "None"))
    (Development|PrintString "SPAWNED SPHERE")))

(event Input|KeyboardEvents|DebugKeyU
  (params (Key :type Key%20Structure :default "None") (ActionValue :type Input%20Action%20Value%20Structure)))

(fn ConstructionScript)