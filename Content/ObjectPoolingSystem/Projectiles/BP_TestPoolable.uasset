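; BP_TestPoolable is a test actor for the object pooling system, reused through activation and deactivation.
; Activate moves it to the pool data's location, unhides it and starts a five-second timer, presumably to trigger deactivation.
; Deactivate parks it far off in the world, hides it and returns it to the pool by class.
; Sphere physics toggles are present but unconnected.
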(event EventBeginPlay)

(event Collision|EventActorBeginOverlap
  (params (OtherActor :type Actor%20Object%20Reference)))

(event EventTick
  (params (DeltaSeconds :type Float%20%28single-precision%29)))

(event EventDeactivate
  (params (ObjectPoolDeactivationData :type Object%20Pool%20Deactivation%20Data%20Structure))
  (bind _self self)
  (Transformation|SetActorLocation "-1000000.000000,0.000000,0.000000" false false)
  (Rendering|SetActorHiddenInGame true)
  (CallFunction|ReturnProjectiletoPool (Utilities|GetClass _self) _self))

(event EventActivate
  (params (ObjectPoolActivationData :type Objec%20Pool%20Activation%20Data%20Structure))
  (Transformation|SetActorLocation (.location (.objectpooltransform ObjectPoolActivationData)) false false)
  (bind _returnvalue (Utilities|Time|SetTimerbyEvent (EventDispatchers|CreateEvent :!event Deactivate) 5.0))
  (Variables|Default|SetTimer%20Handle _returnvalue)
  (Rendering|SetActorHiddenInGame false))

(fn ConstructionScript)

(fn Deactivate
  (Class|Poolable|Deactivate))